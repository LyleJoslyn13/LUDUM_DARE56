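; BP_testEnemy is a test enemy that moves along negative X every Tick by MovementSpeed, without delta-time scaling.
; AnyDamage subtracts health and destroys the actor shortly after health runs out, setting IsDead first.
; Spider-type damage also lowers speed temporarily through a Delay, though its IsSlowed guard is never set true here.
; GetEnemyData exposes the enemy type and death state.
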(event EventBeginPlay)

(event Collision|EventActorBeginOverlap
  (params (OtherActor :type Actor%20Object%20Reference)))

(event EventTick
  (params (DeltaSeconds :type Float%20%28single-precision%29))
  (bind _returnvalue (Transformation|GetActorLocation))
  (Transformation|SetActorLocation (Math|Vector|MakeVector (- (.x _returnvalue) (Variables|Default|GetMovementSpeed)) (.y _returnvalue) (.z _returnvalue)) false false))

(event Game|Damage|EventAnyDamage
  (params (Damage :type Float%20%28single-precision%29) (DamageType :type Damage%20Type%20Object%20Reference) (InstigatedBy :type Controller%20Object%20Reference) (DamageCauser :type Actor%20Object%20Reference))
  (bind _output_get (Variables|Default|SetCurrentHealth (- (Variables|Default|GetCurrentHealth) Damage)))
  (if (== (Variables|Default|GetSpiderDT) (Utilities|GetClass DamageType))
    (Utilities|FlowControl|Sequence
      (:then_0
        ;[1 1 1] STILL NEED SLOWER DAMAGE SPEED
        (if (not (Variables|Default|GetisSlowed))
          (Variables|Default|SetisSlowed false)
          (Variables|Default|SetMovementSpeed 1.0)
          (Utilities|FlowControl|Delay 5.0)
          (Variables|Default|SetMovementSpeed 2.5)))
      (:then_1
        (if (<= _output_get 0.0) :!label _label
          (Variables|Default|SetisDead true)
          (Utilities|FlowControl|Delay 0.1)
          (Actor|DestroyActor))))
    (else
      (goto _label))))

(fn ConstructionScript)

(fn GetEnemyData
  (return (Variables|Default|GetEnemyType) (Variables|Default|GetisDead)))