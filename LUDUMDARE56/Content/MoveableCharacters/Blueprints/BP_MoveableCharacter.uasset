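; BP_MoveableCharacter is a character that moves at a set walk speed and paths to locations on the nav mesh.
; PathToLocation runs AI MoveTo and calls the empty OnTargetReached hook on success.
; Tick watches horizontal velocity to fire the empty OnMovementStopped hook once per stop.
; GetObjectInFrontOfCharacter line-traces forward on Visibility, ignoring all moveable characters, and returns any hit actor.
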(event Custom|PathToLocation
  (params (newPathingLocation :type Vector) (acceptanceRadius :type Float%20%28double-precision%29))
  ;[0.2314 1 0.2314] Move to a location using nav mesh pathfinding
  (AI|AIMoveTo self newPathingLocation 0 acceptanceRadius false
    (:OnSuccess
      (CallFunction|OnTargetReached))))

(event EventBeginPlay
  (Variables|/Script/Engine.CharacterMovementComponent|SetMaxWalkSpeed (Variables|Character|GetCharacterMovement) (Variables|CharacterStats|GetMovementSpeed)))

(event EventTick
  (params (DeltaSeconds :type Float%20%28single-precision%29))
  ;[0.2314 1 0.2314] Check if this actor is moving and if its movement got stopped
  (if (<= (Class|KismetMathLibrary|VSizeXYSquared (Transformation|GetVelocity)) 5.0) ; I'm not moving currently
    (if (Variables|Status|GetIsMoving) ; Was I moving previously?
      (CallFunction|OnMovementStopped) ; This only fires once when this actor stops moving
      (Variables|Status|SetIsMoving false))
    (else
      (Variables|Status|SetIsMoving true))))

(fn ConstructionScript)

(fn OnTargetReached)

(fn OnMovementStopped)

(fn GetObjectinFrontOfCharacter
  (params (TraceRange :type Float%20%28double-precision%29))
  (bind _returnvalue (Transformation|GetActorLocation))
  (bind _outactors (Actor|GetAllActorsOfClass "BP_MoveableCharacter_C"))
  (bind (_outhit _returnvalue_2) (Collision|LineTraceByChannel _returnvalue (+ _returnvalue (* (Transformation|GetActorForwardVector) TraceRange)) "TraceTypeQuery1" false _outactors "ForOneFrame")) ; Line trace in front of the actor to see if something is front of it
  (return _returnvalue_2 (.hitactor _outhit)))