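; BP_TestEnemy is a test enemy character that seeks targets and damages walls and placeholder bugs.
; Each tick it searches for a BP_PlaceholderBug via FindNewTarget, falls back to BP_Base when none is valid, and paths to TargetActor's location.
; AttackTarget calls DamageTarget, which checks the object just in front and applies fixed damage to a TestWall or, with a higher amount, a BP_PlaceholderBug.
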(event EventBeginPlay
  (|CallParentFunction) ; This node is disabled and will not be called.\nDrag off pins to build functionality.
)

(event Collision|EventActorBeginOverlap
  (params (OtherActor :type Actor%20Object%20Reference)))

(event EventTick
  (params (DeltaSeconds :type Float%20%28single-precision%29))
  (|CallParentFunction DeltaSeconds)
  (bind _newtargetactor (CallFunction|FindNewTarget "/Game/MoveableCharacters/Blueprints/BP_PlaceholderBug.BP_PlaceholderBug_C"))
  (if (Utilities|IsValid _newtargetactor)
    _
    (else
      (bind _returnvalue (Actor|GetActorOfClass "/Game/MoveableCharacters/Blueprints/BP_Base.BP_Base_C"))
      (Variables|Default|SetTargetActor _returnvalue)))
  (CallFunction|PathtoLocation (Transformation|GetActorLocation (Variables|Default|GetTargetActor)) 0.0))

(fn ConstructionScript
  (|CallParentFunction))

(fn DamageTarget
  (bind _hitactor (CallFunction|GetObjectinFrontOfCharacter 1e+02))
  (bind _astest_wall (Utilities|Casting|CastToTestWall _hitactor)
    (:then
      (Default|TakeDamage _astest_wall 4e+01))
    (:CastFailed
      (bind _asbp_placeholder_bug (Utilities|Casting|CastToBP_PlaceholderBug _hitactor))
      (Default|TakeDamage _asbp_placeholder_bug 6e+01))))

(fn AttackTarget
  (CallFunction|DamageTarget))