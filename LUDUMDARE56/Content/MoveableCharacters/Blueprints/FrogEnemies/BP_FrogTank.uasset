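; BP_FrogTank is a frog enemy character that chases a target actor and has a smash attack.
; The construction script caches the first BP_PathfindingTestTarget found as TargetActor, and Tick requests a path to that actor's location every frame after running parent logic.
; AttackTarget only plays the FrogTank_Smash montage; nothing in this graph calls it.
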(event EventBeginPlay
  (|CallParentFunction))

(event Collision|EventActorBeginOverlap
  (params (OtherActor :type Actor%20Object%20Reference)))

(event EventTick
  (params (DeltaSeconds :type Float%20%28single-precision%29))
  (|CallParentFunction DeltaSeconds)
  (CallFunction|PathtoLocation (Transformation|GetActorLocation (Variables|Default|GetTargetActor)) 0.0))

(fn ConstructionScript
  (|CallParentFunction)
  (bind _returnvalue (Actor|GetActorOfClass "/Game/MoveableCharacters/Blueprints/BP_PathfindingTestTarget.BP_PathfindingTestTarget_C"))
  (Variables|Default|SetTargetActor _returnvalue))

(fn AttackTarget
  (Animation|PlayAnimMontage "/Game/CharacterAssets/FrogTank/FrogTank_Smash.FrogTank_Smash" 1.0 "None"))