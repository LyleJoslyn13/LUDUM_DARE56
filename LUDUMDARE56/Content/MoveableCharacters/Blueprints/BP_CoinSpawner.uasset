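; BP_CoinSpawner scatters BP_Coin pickups around its location when play begins.
; SpawnCoins loops up to CoinsToSpawn, calling SpawnCoin to place each coin at a random reachable navmesh point within SpawnRadius.
; Spawning adjusts for collisions where possible but always creates the coin.
; The construction script sizes VisualizerSphere to SpawnRadius to show the spawn area.
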(event EventBeginPlay
  (CallFunction|SpawnCoins))

(event Collision|EventActorBeginOverlap
  (params (OtherActor :type Actor%20Object%20Reference)))

(event EventTick
  (params (DeltaSeconds :type Float%20%28single-precision%29)))

(fn ConstructionScript
  (Components|Sphere|SetSphereRadius (Variables|Default|GetVisualizerSphere) (Variables|Default|GetSpawnRadius) true))

(fn SpawnCoin
  (Game|SpawnActorfromClass "/Game/Coins/BP_Coin.BP_Coin_C" (Math|Conversions|ToTransform(Vector) (.RandomLocation (AI|Navigation|GetRandomReachablePointinRadius (Transformation|GetActorLocation) (Variables|Default|GetSpawnRadius) 0 "/Script/AIModule.NavFilter_AIControllerDefault"))) "AdjustIfPossibleButAlwaysSpawn" "MultiplyWithRoot" 0 0)
  (return))

(fn SpawnCoins
  (for _index (range 0 (Variables|Default|GetCoinsToSpawn))
    (CallFunction|SpawnCoin)))