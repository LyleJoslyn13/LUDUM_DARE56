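; BP_AnthillAnt is a temporary attacker ant that chases an enemy target, damages it, then returns to its spawn point and despawns.
; Tick paths toward EnemyTarget and attacks in range, throttled by an AttackRate cooldown.
; It heads home when its attacks run out or TimeoutTime elapses, and destroys itself when it stops near spawn.
; A further Lifetime delay after the timeout destroys it as a fallback.
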(event Custom|AttackCooldown
  (Utilities|FlowControl|Delay (/ 1.0 (Variables|Default|GetAttackRate)))
  (Variables|Default|SetAttacking false))

(event EventBeginPlay
  (|CallParentFunction)
  (Utilities|FlowControl|Delay (Variables|Default|GetTimeoutTime))
  (CallFunction|ReturntoSpawn)
  (Utilities|FlowControl|Delay (Variables|Default|GetLifetime))
  (Actor|DestroyActor))

(event EventTick
  (params (DeltaSeconds :type Float%20%28single-precision%29))
  (|CallParentFunction DeltaSeconds)
  (if (and (not (Variables|Default|GetReturning)) (Utilities|IsValid (Variables|Default|GetEnemyTarget)))
    (CallFunction|PathtoLocation (Transformation|GetActorLocation (Variables|Default|GetEnemyTarget)) 0.0)
    (if (and (not (Variables|Default|GetAttacking)) (<= (Transformation|GetDistanceTo (Variables|Default|GetEnemyTarget)) (Variables|Default|GetAttackRange)))
      (Variables|Default|SetAttacking true)
      (CallFunction|AttackTarget)
      (CallFunction|AttackCooldown))))

(fn ConstructionScript
  (|CallParentFunction)
  (Variables|Default|SetSpawnLocation (Transformation|GetActorLocation)))

(fn ReturntoSpawn
  (Variables|Default|SetReturning true)
  (CallFunction|PathtoLocation (Variables|Default|GetSpawnLocation) 2e+02)
  (CallFunction|OnMovementStopped))

(fn OnMovementStopped
  (|CallParentFunction)
  (if (and (<= (Math|Vector|Distance(Vector) (Transformation|GetActorLocation) (Variables|Default|GetSpawnLocation)) 3e+02) (Variables|Default|GetReturning))
    (Actor|DestroyActor)))

(fn AttackTarget
  (bind _result (Math|Integer|DecrementInt (Variables|Default|GetAttacksRemaining))
    (:%20%20
      (Default|TakeDamage (Variables|Default|GetEnemyTarget) (Variables|Default|GetDamage) false)
      (if (<= _result 0)
        (CallFunction|ReturntoSpawn)))))