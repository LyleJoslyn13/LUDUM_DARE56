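; Enemy character Blueprint that hunts the nearest placeholder bug, falling back to the base when none remain.
; Each tick it updates cooldown and target distance, attacking when in range or stopped; AttackTarget only prints here.
; A forward hit check locks it onto the base and picks whether DamageTarget hurts a wall, bug or base.
; At zero health it removes itself from the phase manager and is destroyed.
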(event EventTick
  (params (DeltaSeconds :type Float%20%28single-precision%29))
  (CallFunction|UpdateAttackCooldown DeltaSeconds) ; Decrease attack cooldown
  (if (Variables|Status|GetAttackingBase)
    (CallFunction|CheckifCanAttack true)
    (CallFunction|AimatTarget)
    (else
      (CallFunction|StandardTargetPriority) ; Target bugs then base
      (CallFunction|UpdateTargetInfo) ; Update info about my target actor
      (CallFunction|CheckifCanAttack false) ; Can I attack this tick?
      (CallFunction|BaseTargeting) ; Can I attack the base?
    ))
  (|CallParentFunction DeltaSeconds))

(fn ConstructionScript
  (|CallParentFunction)
  (bind _newtargetactor (CallFunction|FindNewTarget "/Game/MoveableCharacters/Blueprints/Placeholders/BP_PlaceholderBug.BP_PlaceholderBug_C"))
  (Variables|Status|SetTargetActor _newtargetactor)
  (bind _returnvalue (Actor|GetActorOfClass "/Game/MoveableCharacters/Blueprints/BP_PhaseManager.BP_PhaseManager_C"))
  (Variables|Default|SetPhaseManager _returnvalue))

(fn FindNewTarget
  (params (TargetClass :type Actor%20Class%20Reference))
  (bind _outactors (Actor|GetAllActorsOfClass TargetClass))
  (bind _output_get (Variables|Status|SetTargetActor (.ReturnValue (Actor|FindNearestActor (Transformation|GetActorLocation) _outactors))))
  (return _output_get))

(fn TakeDamage
  (params (damage :type Float%20%28double-precision%29))
  (if (not (Variables|Status|GetisDead)) ; Don't let enemies take damage after death in case we add damage effects
    (bind _output_get (Variables|CharacterStats|SetCurrentHealth (- (Variables|CharacterStats|GetCurrentHealth) damage)))
    (if (<= _output_get 0.0)
      (CallFunction|DeathSequence))))

(fn FindNearestActorinArray)

(fn UpdateTargetInfo
  (bind _targetactor (Variables|Status|GetTargetActor))
  (if (Utilities|IsValid _targetactor)
    (Variables|Status|SetDistanceToTarget (Transformation|GetDistanceTo _targetactor))))

(fn AttackTarget
  (Development|PrintString "Attack!"))

(fn DamageTarget
  (bind _hitactor (CallFunction|GetObjectinFrontOfCharacter (Variables|CharacterStats|GetAttackRange)))
  (bind _astest_wall (Utilities|Casting|CastToTestWall _hitactor)
    (:then
      (Default|TakeDamage _astest_wall (Variables|CharacterStats|GetWallDamage)))
    (:CastFailed
      (bind _asbp_placeholder_bug (Utilities|Casting|CastToBP_PlaceholderBug _hitactor)
        (:then
          (Default|TakeDamage _asbp_placeholder_bug (Variables|CharacterStats|GetDamage)))
        (:CastFailed
          (bind _asbp_base (Utilities|Casting|CastToBP_Base _hitactor))
          (Default|TakeDamage _asbp_base (Variables|CharacterStats|GetDamage)))))))

(fn UpdateAttackCooldown
  (params (deltaTime :type Float%20%28double-precision%29))
  (Variables|Status|SetAttackCooldown (Math|Float|Clamp(Float) (- (Variables|Status|GetAttackCooldown) deltaTime) 0.0 (Variables|Status|GetAttackCooldown))))

(fn CheckifCanAttack
  (params (Override :type Boolean))
  (if (Math|Boolean|ANDBoolean (Utilities|IsValid (Variables|Status|GetTargetActor)) (<= (Variables|Status|GetAttackCooldown) 0.0) (or (or (<= (Variables|Status|GetDistanceToTarget) (Variables|CharacterStats|GetAttackRange)) (not (Variables|Default|GetIsMoving))) Override)) ; Can I attack?
    (Components|Movement|StopMovementImmediately (Variables|Character|GetCharacterMovement))
    (Variables|Status|SetAttackCooldown (/ 1.0 (Variables|CharacterStats|GetAttackSpeed)))
    (CallFunction|AttackTarget)))

(fn DeathSequence
  (Variables|Status|SetisDead true)
  (Default|RemoveDeadEnemy (Variables|Default|GetPhaseManager) self)
  (Actor|DestroyActor))

(fn StandardTargetPriority
  (if (not (Utilities|IsValid (Variables|Status|GetTargetActor)))
    (bind _newtargetactor (CallFunction|FindNewTarget "/Game/MoveableCharacters/Blueprints/Placeholders/BP_PlaceholderBug.BP_PlaceholderBug_C"))
    (if (Utilities|IsValid _newtargetactor)
      (Variables|Status|SetTargetActor _newtargetactor)
      (else
        (bind _returnvalue (Actor|GetActorOfClass "/Game/MoveableCharacters/Blueprints/BP_Base.BP_Base_C"))
        (Variables|Status|SetTargetActor _returnvalue)))))

(fn BaseTargeting
  (if (== (Utilities|GetClass (Variables|Status|GetTargetActor)) "/Game/MoveableCharacters/Blueprints/BP_Base.BP_Base_C")
    (bind _hitactor (CallFunction|GetObjectinFrontOfCharacter (Variables|CharacterStats|GetAttackRange)))
    (if (== _hitactor (Variables|Status|GetTargetActor))
      (Variables|Status|SetAttackingBase true))))

(fn AimatTarget
  (Transformation|SetWorldRotation (Variables|Default|GetCapsuleComponent) (Math|Rotator|FindLookatRotation (Transformation|GetActorLocation) (Transformation|GetActorLocation (Variables|Status|GetTargetActor))) false false)
  (CallFunction|CheckifCanAttack false))