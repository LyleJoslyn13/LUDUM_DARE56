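; BP_TestTankEnemy is a test tank enemy that continually paths toward the base actor.
; Each Tick, after calling the parent, it finds a BP_Base with GetActorOfClass, stores it as TargetActor, and passes its location to PathToLocation with zero acceptance radius.
; The lookup and path request repeat every frame rather than being cached.
; The construction script only calls its parent.
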(event EventBeginPlay
  (|CallParentFunction) ; This node is disabled and will not be called.\nDrag off pins to build functionality.
)

(event Collision|EventActorBeginOverlap
  (params (OtherActor :type Actor%20Object%20Reference))
  (|CallParentFunction OtherActor) ; This node is disabled and will not be called.\nDrag off pins to build functionality.
)

(event EventTick
  (params (DeltaSeconds :type Float%20%28single-precision%29))
  (|CallParentFunction DeltaSeconds)
  (bind _returnvalue (Actor|GetActorOfClass "/Game/MoveableCharacters/Blueprints/BP_Base.BP_Base_C"))
  (Variables|Default|SetTargetActor _returnvalue)
  (CallFunction|PathtoLocation (Transformation|GetActorLocation (Variables|Default|GetTargetActor)) 0.0))

(fn ConstructionScript
  (|CallParentFunction))