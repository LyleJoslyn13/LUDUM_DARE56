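; Placeholder anthill bug actor that spawns attacking ants at its own location when an enemy comes within detection range.
; Every tick it searches all BP_EnemyCharacter actors for the nearest one and stores it as Target, clearing Target when none qualifies.
; A valid target spawns a BP_AnthillAnt with that enemy as EnemyTarget, gated by a CanSpawnAnt flag that resets after the AttackCD delay.
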(event Custom|WaitForAttackCD
  (Utilities|FlowControl|Delay (Variables|Default|GetAttackCD))
  (Variables|Default|SetCanSpawnAnt true))

(event EventBeginPlay
  (|CallParentFunction) ; This node is disabled and will not be called.\nDrag off pins to build functionality.
)

(event Collision|EventActorBeginOverlap
  (params (OtherActor :type Actor%20Object%20Reference))
  (|CallParentFunction OtherActor) ; This node is disabled and will not be called.\nDrag off pins to build functionality.
)

(event EventTick
  (params (DeltaSeconds :type Float%20%28single-precision%29))
  (|CallParentFunction DeltaSeconds)
  (bind _outactors (Actor|GetAllActorsOfClass "/Game/MoveableCharacters/Blueprints/BP_EnemyCharacter.BP_EnemyCharacter_C"))
  (if (<= (.Distance (Actor|FindNearestActor (Transformation|GetActorLocation) _outactors)) (Variables|Default|GetDetectionRange))
    (bind _asbp_enemy_character (Utilities|Casting|CastToBP_EnemyCharacter (.ReturnValue (Actor|FindNearestActor (Transformation|GetActorLocation) _outactors)))
      (:then
        (bind _output_get (Variables|Default|SetTarget _asbp_enemy_character))
        (if (and (Utilities|IsValid _output_get) (Variables|Default|GetCanSpawnAnt))
          (Variables|Default|SetCanSpawnAnt false)
          (Game|SpawnActorfromClass "/Game/MoveableCharacters/Blueprints/OtherCharacters/BP_AnthillAnt.BP_AnthillAnt_C" (Math|Conversions|ToTransform(Vector) (Transformation|GetActorLocation)) "AdjustIfPossibleButAlwaysSpawn" "MultiplyWithRoot" 0 (Variables|Default|GetTarget) 0)
          (CallFunction|WaitforAttackCD)))
      (:CastFailed
        (Variables|Default|SetTarget 0 :!label _label)))
    (else
      (goto _label))))

(fn ConstructionScript
  (|CallParentFunction))