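; Game phase manager that alternates a timed search phase with an attack phase of frog enemy waves.
; Tick counts down the search timer to start an attack, or returns to search once spawning finishes and the enemy list empties via RemoveDeadEnemy.
; SpawnWave runs four scripted, delayed waves, then endless waves scaled by WaveCounter.
; SpawnGroup picks random BP_WaveSpawner actors, cached in the Construction Script, and tracks each spawned enemy.
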(event Custom|TestWave
  (Utilities|FlowControl|Delay 2.0)
  (CallFunction|SpawnGroup "/Game/MoveableCharacters/Blueprints/FrogEnemies/BP_FrogMelee.BP_FrogMelee_C" 3)
  (Utilities|FlowControl|Delay 4.0)
  (CallFunction|SpawnGroup "/Game/MoveableCharacters/Blueprints/FrogEnemies/BP_FrogMelee.BP_FrogMelee_C" 2)
  (Utilities|FlowControl|Delay 4.0)
  (CallFunction|SpawnGroup "/Game/MoveableCharacters/Blueprints/FrogEnemies/BP_FrogTank.BP_FrogTank_C" 2)
  (CallFunction|SpawnGroup "/Game/MoveableCharacters/Blueprints/FrogEnemies/BP_FrogRanged.BP_FrogRanged_C" 2)
  (Utilities|FlowControl|Delay 4.0)
  (CallFunction|SpawnGroup "/Game/MoveableCharacters/Blueprints/FrogEnemies/BP_FrogTank.BP_FrogTank_C" 2))

(event Custom|SpawnWave
  (Variables|Default|SetspawningFinished false)
  (switch int (Variables|Default|GetwaveCounter)
    (:Default
      ;[1 1 1] Infinite wave
      (Utilities|FlowControl|Delay 3.0)
      (CallFunction|SpawnGroup "/Game/MoveableCharacters/Blueprints/FrogEnemies/BP_FrogMelee.BP_FrogMelee_C" (* 1.2 (Variables|Default|GetwaveCounter)))
      (Variables|Default|SetspawnStart true)
      (CallFunction|SpawnGroup "/Game/MoveableCharacters/Blueprints/FrogEnemies/BP_FrogTank.BP_FrogTank_C" (* 0.7 (Variables|Default|GetwaveCounter)))
      (Utilities|FlowControl|Delay 6.0)
      (CallFunction|SpawnGroup "/Game/MoveableCharacters/Blueprints/FrogEnemies/BP_FrogMelee.BP_FrogMelee_C" (* 1.0 (Variables|Default|GetwaveCounter)))
      (CallFunction|SpawnGroup "/Game/MoveableCharacters/Blueprints/FrogEnemies/BP_FrogRanged.BP_FrogRanged_C" (* 1.4 (Variables|Default|GetwaveCounter)))
      (Utilities|FlowControl|Delay 6.0)
      (CallFunction|SpawnGroup "/Game/MoveableCharacters/Blueprints/FrogEnemies/BP_FrogTank.BP_FrogTank_C" (* 1.3 (Variables|Default|GetwaveCounter)))
      (CallFunction|SpawnGroup "/Game/MoveableCharacters/Blueprints/FrogEnemies/BP_FrogMelee.BP_FrogMelee_C" (* 1.0 (Variables|Default|GetwaveCounter)))
      (Utilities|FlowControl|Delay 6.0)
      (CallFunction|SpawnGroup "/Game/MoveableCharacters/Blueprints/FrogEnemies/BP_FrogRanged.BP_FrogRanged_C" (* 1.0 (Variables|Default|GetwaveCounter)))
      (CallFunction|SpawnGroup "/Game/MoveableCharacters/Blueprints/FrogEnemies/BP_FrogMelee.BP_FrogMelee_C" (* 1.0 (Variables|Default|GetwaveCounter)))
      (Utilities|FlowControl|Delay 6.0)
      (CallFunction|SpawnGroup "/Game/MoveableCharacters/Blueprints/FrogEnemies/BP_FrogTank.BP_FrogTank_C" (* 1.5 (Variables|Default|GetwaveCounter)))
      (CallFunction|SpawnGroup "/Game/MoveableCharacters/Blueprints/FrogEnemies/BP_FrogRanged.BP_FrogRanged_C" (* 2.0 (Variables|Default|GetwaveCounter)))
      (Variables|Default|SetspawningFinished true))
    (:0
      ;[1 1 1] Wave1
      (Utilities|FlowControl|Delay 5.0)
      (CallFunction|SpawnGroup "/Game/MoveableCharacters/Blueprints/FrogEnemies/BP_FrogMelee.BP_FrogMelee_C" 2)
      (Variables|Default|SetspawnStart true)
      (Utilities|FlowControl|Delay 8.0)
      (CallFunction|SpawnGroup "/Game/MoveableCharacters/Blueprints/FrogEnemies/BP_FrogMelee.BP_FrogMelee_C" 3)
      (Utilities|FlowControl|Delay 1e+01)
      (CallFunction|SpawnGroup "/Game/MoveableCharacters/Blueprints/FrogEnemies/BP_FrogMelee.BP_FrogMelee_C" 2)
      (Variables|Default|SetspawningFinished true))
    (:1
      ;[1 1 1] Wave2
      (Utilities|FlowControl|Delay 5.0)
      (CallFunction|SpawnGroup "/Game/MoveableCharacters/Blueprints/FrogEnemies/BP_FrogMelee.BP_FrogMelee_C" 4)
      (Variables|Default|SetspawnStart true)
      (Utilities|FlowControl|Delay 8.0)
      (CallFunction|SpawnGroup "/Game/MoveableCharacters/Blueprints/FrogEnemies/BP_FrogMelee.BP_FrogMelee_C" 3)
      (CallFunction|SpawnGroup "/Game/MoveableCharacters/Blueprints/FrogEnemies/BP_FrogRanged.BP_FrogRanged_C" 2)
      (Utilities|FlowControl|Delay 8.0)
      (CallFunction|SpawnGroup "/Game/MoveableCharacters/Blueprints/FrogEnemies/BP_FrogMelee.BP_FrogMelee_C" 3)
      (Variables|Default|SetspawningFinished true))
    (:2
      ;[1 1 1] Wave 3
      (Utilities|FlowControl|Delay 4.0)
      (CallFunction|SpawnGroup "/Game/MoveableCharacters/Blueprints/FrogEnemies/BP_FrogMelee.BP_FrogMelee_C" 5)
      (Variables|Default|SetspawnStart true)
      (Utilities|FlowControl|Delay 6.0)
      (CallFunction|SpawnGroup "/Game/MoveableCharacters/Blueprints/FrogEnemies/BP_FrogMelee.BP_FrogMelee_C" 2)
      (CallFunction|SpawnGroup "/Game/MoveableCharacters/Blueprints/FrogEnemies/BP_FrogTank.BP_FrogTank_C" 2)
      (Utilities|FlowControl|Delay 6.0)
      (CallFunction|SpawnGroup "/Game/MoveableCharacters/Blueprints/FrogEnemies/BP_FrogRanged.BP_FrogRanged_C" 3)
      (Variables|Default|SetspawningFinished true))
    (:3
      ;[1 1 1] Wave 4
      (Utilities|FlowControl|Delay 3.0)
      (CallFunction|SpawnGroup "/Game/MoveableCharacters/Blueprints/FrogEnemies/BP_FrogMelee.BP_FrogMelee_C" 4)
      (Variables|Default|SetspawnStart true)
      (CallFunction|SpawnGroup "/Game/MoveableCharacters/Blueprints/FrogEnemies/BP_FrogTank.BP_FrogTank_C" 2)
      (Utilities|FlowControl|Delay 6.0)
      (CallFunction|SpawnGroup "/Game/MoveableCharacters/Blueprints/FrogEnemies/BP_FrogMelee.BP_FrogMelee_C" 3)
      (CallFunction|SpawnGroup "/Game/MoveableCharacters/Blueprints/FrogEnemies/BP_FrogRanged.BP_FrogRanged_C" 5)
      (Utilities|FlowControl|Delay 6.0)
      (CallFunction|SpawnGroup "/Game/MoveableCharacters/Blueprints/FrogEnemies/BP_FrogTank.BP_FrogTank_C" 4)
      (CallFunction|SpawnGroup "/Game/MoveableCharacters/Blueprints/FrogEnemies/BP_FrogMelee.BP_FrogMelee_C" 3)
      (Utilities|FlowControl|Delay 6.0)
      (CallFunction|SpawnGroup "/Game/MoveableCharacters/Blueprints/FrogEnemies/BP_FrogRanged.BP_FrogRanged_C" 3)
      (CallFunction|SpawnGroup "/Game/MoveableCharacters/Blueprints/FrogEnemies/BP_FrogMelee.BP_FrogMelee_C" 3)
      (Variables|Default|SetspawningFinished true))))

(event EventTick
  (params (DeltaSeconds :type Float%20%28single-precision%29))
  (if (Variables|Default|GetattackPhase)
    (CallFunction|CheckforWaveEnd)
    (else
      (CallFunction|DecreaseSearchTimer DeltaSeconds))))

(event EventBeginPlay
  (CallFunction|SwitchtoSearchPhase))

(fn ConstructionScript
  (bind _outactors (Actor|GetAllActorsOfClass "/Game/MoveableCharacters/Blueprints/BP_WaveSpawner.BP_WaveSpawner_C"))
  (Variables|Default|SetwaveSpawners _outactors))

(fn SpawnGroup
  (params (ClassToSpawn :type BP%20Enemy%20Character%20Class%20Reference) (NumberToSpawn :type Integer))
  (for _index (range 0 NumberToSpawn)
    (bind _newenemy (Default|SpawnEnemyWithinRadius (.OutItem (Utilities|Array|Random (Variables|Default|GetwaveSpawners))) ClassToSpawn))
    (Utilities|Array|Add (Variables|Default|GetcurrentEnemies) _newenemy)))

(fn SwitchtoSearchPhase
  (Development|PrintString "Search time!")
  (Variables|Default|SetattackPhase false)
  (Variables|Default|SetsearchTimer (Variables|Default|GetsearchMaxTime)))

(fn SwitchtoAttackPhase
  (Variables|Default|SetattackPhase true)
  (CallFunction|SpawnWave)
  (Development|PrintString "Attack time!! >:)"))

(fn DecreaseSearchTimer
  (params (deltaTime :type Float%20%28double-precision%29))
  (bind _output_get (Variables|Default|SetsearchTimer (- (Variables|Default|GetsearchTimer) deltaTime)))
  (if (<= _output_get 0.0)
    (CallFunction|SwitchtoAttackPhase)))

(fn CheckforWaveEnd
  (bind _currentenemies (Variables|Default|GetcurrentEnemies))
  (bind _returnvalue (Utilities|Array|Length _currentenemies))
  (Development|PrintString (Utilities|String|ToString(Integer) _returnvalue))
  (if (and (<= _returnvalue 0) (Variables|Default|GetspawningFinished))
    (Math|Integer|IncrementInt (Variables|Default|GetwaveCounter)
      (:%20%20
        (CallFunction|SwitchtoSearchPhase)
        (Variables|Default|SetspawnStart false)))))

(fn RemoveDeadEnemy
  (params (EnemyToRemove :type BP%20Enemy%20Character%20Object%20Reference))
  (Utilities|Array|RemoveItem (Variables|Default|GetcurrentEnemies) EnemyToRemove))