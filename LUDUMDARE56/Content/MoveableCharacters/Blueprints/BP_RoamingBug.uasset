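; Roaming bug character that wanders the nav mesh, runs from the player and is destroyed when caught.
; Tick updates player distance and dot product to detect the player by forward sight cone or near radius, and starts roaming when idle.
; Roaming alternates random reachable destinations with timed pauses.
; Detection triggers a delayed, faster flight to a nav-projected point away from the player, ended by cooldown or movement stopping.
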(event Custom|FleeingCooldown
  (Utilities|FlowControl|Delay (Variables|CharacterStats|GetFleeCooldown))
  (Components|Movement|StopMovementImmediately (Variables|Character|GetCharacterMovement))
  (Variables|Status|SetFleeing false)
  (Variables|/Script/Engine.CharacterMovementComponent|SetMaxWalkSpeed (Variables|Character|GetCharacterMovement) (Variables|Default|GetMovementSpeed)))

(event Custom|AlertBug
  (Components|Movement|StopMovementImmediately (Variables|Character|GetCharacterMovement))
  (Variables|Status|SetFleeing true)
  (Variables|Status|SetRoaming false)
  (Utilities|FlowControl|Delay (Variables|CharacterStats|GetDetectionTime))
  (CallFunction|FleefromPlayer))

(event Custom|WaitForRoamingEnd
  (Utilities|FlowControl|Delay (Math|Random|RandomFloatinRange 3.0 8.0))
  (if (not (Variables|Status|GetFleeing))
    (Components|Movement|StopMovementImmediately (Variables|Character|GetCharacterMovement))
    (Utilities|FlowControl|Delay (Math|Random|RandomFloatinRange 2.0 3.0))
    (Variables|Status|SetRoaming false)))

(event EventTick
  (params (DeltaSeconds :type Float%20%28single-precision%29))
  (CallFunction|UpdatePlayerInfo)
  (CallFunction|SearchforPlayer)
  (if (and (not (Variables|Status|GetRoaming)) (not (Variables|Status|GetFleeing)))
    (CallFunction|RoamtoNewLocation)))

(fn ConstructionScript
  (|CallParentFunction))

(fn FleefromPlayer
  (bind _returnvalue (Transformation|GetActorLocation))
  (bind _fleeingdistance (Variables|CharacterStats|GetFleeingDistance))
  (Variables|/Script/Engine.CharacterMovementComponent|SetMaxWalkSpeed (Variables|Character|GetCharacterMovement) (Variables|CharacterStats|GetFleeingSpeed))
  (CallFunction|PathtoLocation (.ProjectedLocation (AI|Navigation|ProjectPointtoNavigation (+ (* (Math|Vector|GetForwardVector (Math|Rotator|FindLookatRotation (Transformation|GetActorLocation (Game|GetPlayerCharacter 0)) _returnvalue)) _fleeingdistance) _returnvalue) 0 "/Script/AIModule.NavFilter_AIControllerDefault" (Math|Conversions|ToVector(Float) _fleeingdistance))) 0.0)
  (CallFunction|FleeingCooldown))

(fn SearchforPlayer
  (bind _distancetoplayer (Variables|Status|GetDistanceToPlayer))
  (if (and (not (Variables|Status|GetFleeing)) (Utilities|IsValid (Game|GetPlayerCharacter 0)))
    (if (or (and (> (Variables|Status|GetDotProdToPlayer) 0.5) (<= _distancetoplayer (Variables|CharacterStats|GetSightRadius))) (<= _distancetoplayer (Variables|CharacterStats|GetNearDetectionRadius))) ; I need to run away!!
      (CallFunction|AlertBug))))

(fn UpdatePlayerInfo
  (bind _returnvalue (Game|GetPlayerCharacter 0))
  (if (Utilities|IsValid _returnvalue)
    (Variables|Status|SetDistanceToPlayer (Transformation|GetDistanceTo _returnvalue))
    (Variables|Status|SetDotProdToPlayer (Class|Actor|GetDotProductto _returnvalue))))

(fn CatchBug
  (Actor|DestroyActor))

(fn RoamtoNewLocation
  (Variables|Status|SetRoaming true)
  (CallFunction|PathtoLocation (.RandomLocation (AI|Navigation|GetRandomReachablePointinRadius (Transformation|GetActorLocation) (Variables|CharacterStats|GetRoamingRange) 0 "/Script/AIModule.NavFilter_AIControllerDefault")) 0.0)
  (CallFunction|WaitforRoamingEnd))

(fn OnMovementStopped
  (|CallParentFunction)
  (Variables|Status|SetFleeing false))