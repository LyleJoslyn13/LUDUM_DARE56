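; Child spider tower in the bug tower set that aims at a targeted enemy and shoots webs.
; ShootTarget re-aims the Arrow each tick through a delay loop, spawning BP_ChildWeb with a one-second cooldown until the target dies or is cleared.
; Leaving the range collision clears that target.
; Target selection favouring enemy type 2 (tank) is disconnected, so entering range only casts and never starts shooting here.
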(event OnComponentBeginOverlap(RangeCollision)
  (params (OverlappedComponent :type Primitive%20Component%20Object%20Reference) (OtherActor :type Actor%20Object%20Reference) (OtherComp :type Primitive%20Component%20Object%20Reference) (OtherBodyIndex :type Integer) (bFromSweep :type Boolean) (SweepResult :type Hit%20Result%20Structure%20%28by%20ref%29))
  (bind _asbp_test_enemy (Utilities|Casting|CastToBP_testEnemy OtherActor)))

(event OnComponentEndOverlap(RangeCollision)
  (params (OverlappedComponent :type Primitive%20Component%20Object%20Reference) (OtherActor :type Actor%20Object%20Reference) (OtherComp :type Primitive%20Component%20Object%20Reference) (OtherBodyIndex :type Integer))
  (if (== OtherActor (Variables|Default|GetTargetedActor))
    (Variables|Default|SetIsTargeted false)
    (if (Variables|Default|GetisPrimaryTarget)
      (Variables|Default|SetisPrimaryTarget false))))

(event Custom|ShootTarget
  (bind _targetedactor (Variables|Default|GetTargetedActor))
  (bind _arrow (Variables|Default|GetArrow))
  (bind _returnvalue (Transformation|GetWorldLocation _arrow))
  (if (Variables|Default|GetIsTargeted) :!label _label
    (bind _isdead (Class|BPIEnemyData|GetEnemyData(Message) _targetedactor))
    (if _isdead
      (Variables|Default|SetIsTargeted false)
      (else
        (Transformation|SetWorldRotation _arrow (Math|Rotator|FindLookatRotation _returnvalue (Transformation|GetWorldLocation (Variables|/Script/Engine.Actor|GetRootComponent _targetedactor))) false false)
        (Utilities|FlowControl|Sequence
          (:then_0
            (Utilities|FlowControl|DelayUntilNextTick)
            (goto _label))
          (:then_1
            (if (not (Variables|Default|GetisAttacking))
              (Variables|Default|SetisAttacking true)
              (Game|SpawnActorfromClass "/Game/Bugs/BugTowerActors/BP_ChildWeb.BP_ChildWeb_C" (Math|Transform|MakeTransform _returnvalue (Math|Conversions|RotationFromXVector (Math|Vector|GetForwardVector _arrow)) "1.000000,1.000000,1.000000") "Undefined" "MultiplyWithRoot" 0 0)
              (Utilities|FlowControl|Delay 1.0)
              (Variables|Default|SetisAttacking false))))))))

(event EventBeginPlay
  (|CallParentFunction) ; This node is disabled and will not be called.\nDrag off pins to build functionality.
)

(event Collision|EventActorBeginOverlap
  (params (OtherActor :type Actor%20Object%20Reference))
  (|CallParentFunction OtherActor) ; This node is disabled and will not be called.\nDrag off pins to build functionality.
)

(event EventTick
  (params (DeltaSeconds :type Float%20%28single-precision%29))
  (|CallParentFunction DeltaSeconds) ; This node is disabled and will not be called.\nDrag off pins to build functionality.
)

(fn ConstructionScript
  (|CallParentFunction))