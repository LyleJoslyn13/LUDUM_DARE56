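; BP_ChildAnthill is a bug tower actor that spawns BP_AnthillAnt actors to attack its current Target.
; Each tick it eases its yaw toward the target and, when off cooldown, spawns an ant at SpawnPoint with that enemy assigned.
; A delay of AttackCD re-arms spawning, and construction sizes RangeCollision from DetectionRange0.
; CheckForTarget0 runs every tick but is empty, so this graph never assigns Target itself.
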(event Custom|WaitForAttackCD
  (Utilities|FlowControl|Delay (Variables|Default|GetAttackCD))
  (Variables|Default|SetCanSpawnAnt true))

(event EventBeginPlay
  (|CallParentFunction) ; This node is disabled and will not be called.\nDrag off pins to build functionality.
)

(event Collision|EventActorBeginOverlap
  (params (OtherActor :type Actor%20Object%20Reference))
  (|CallParentFunction OtherActor) ; This node is disabled and will not be called.\nDrag off pins to build functionality.
)

(event EventTick
  (params (DeltaSeconds :type Float%20%28single-precision%29))
  (|CallParentFunction DeltaSeconds)
  (CallFunction|CheckforTarget0)
  (CallFunction|RotateTowardsTarget)
  (if (and (Utilities|IsValid (Variables|Default|GetTarget)) (Variables|Default|GetCanSpawnAnt))
    (Variables|Default|SetCanSpawnAnt false)
    (Game|SpawnActorfromClass "/Game/MoveableCharacters/Blueprints/OtherCharacters/BP_AnthillAnt.BP_AnthillAnt_C" (Math|Conversions|ToTransform(Vector) (Transformation|GetWorldLocation (Variables|Default|GetSpawnPoint))) "AdjustIfPossibleButAlwaysSpawn" "MultiplyWithRoot" 0 (Variables|Default|GetTarget) 0)
    (CallFunction|WaitforAttackCD)))

(fn ConstructionScript
  (|CallParentFunction)
  (Components|Sphere|SetSphereRadius (Variables|Default|GetRangeCollision) (Variables|Default|GetdetectionRange_0) true))

(fn CheckforTarget0)

(fn RotateTowardsTarget
  (if (Utilities|IsValid (Variables|Default|GetTarget))
    (Transformation|SetWorldRotation (Variables|Default|GetDefaultSceneRoot) (Math|Rotator|MakeRotator 0.0 0.0 (Math|Float|Lerp (.yaw (Transformation|GetWorldRotation (Variables|Default|GetDefaultSceneRoot))) (.yaw (Math|Rotator|FindLookatRotation (Transformation|GetActorLocation) (Transformation|GetActorLocation (Variables|Default|GetTarget)))) 0.1)) false false)))