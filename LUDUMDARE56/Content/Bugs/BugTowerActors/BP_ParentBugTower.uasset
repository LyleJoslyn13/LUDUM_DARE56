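; Base bug tower actor that targets and turns to face enemy characters, with health that destroys it at zero.
; Each tick without a valid target, it scans all BP_EnemyCharacter actors and takes the nearest within AttackRange.
; It keeps that target until invalid, rotating its root toward it without rechecking range.
; AttackRange also sizes the range sphere at construction, though targeting uses distance checks; no attack logic is implemented here.
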(event EventBeginPlay)

(event Collision|EventActorBeginOverlap
  (params (OtherActor :type Actor%20Object%20Reference)))

(event EventTick
  (params (DeltaSeconds :type Float%20%28single-precision%29))
  (if (Utilities|IsValid (Variables|Default|GetTargetedActor))
    (Transformation|SetWorldRotation (Variables|Default|GetDefaultSceneRoot) (Math|Rotator|FindLookatRotation (Transformation|GetActorLocation) (Transformation|GetActorLocation (Variables|Default|GetTargetedActor))) false false)
    (else
      (CallFunction|CheckforTarget))))

(fn ConstructionScript
  (Components|Sphere|SetSphereRadius (Variables|Default|GetRangeCollision) (Variables|Default|GetattackRange) true))

(fn TakeDamage
  (params (Damage :type Float%20%28double-precision%29))
  (bind _output_get (Variables|Default|Sethealth (- (Variables|Default|Gethealth) Damage)))
  (if (<= _output_get 0.0)
    (Actor|DestroyActor)))

(fn CheckforTarget
  (if (not (Utilities|IsValid (Variables|Default|GetTargetedActor)))
    (bind _outactors (Actor|GetAllActorsOfClass "/Game/MoveableCharacters/Blueprints/BP_EnemyCharacter.BP_EnemyCharacter_C"))
    (if (<= (.Distance (Actor|FindNearestActor (Transformation|GetActorLocation) _outactors)) (Variables|Default|GetattackRange))
      (bind _asbp_enemy_character (Utilities|Casting|CastToBP_EnemyCharacter (.ReturnValue (Actor|FindNearestActor (Transformation|GetActorLocation) _outactors))))
      (Variables|Default|SetTargetedActor _asbp_enemy_character)
      (else
        (Variables|Default|SetTargetedActor 0)))))

(fn GetEnemyData
  (return 0 false))

(fn GetTargetedActor
  (return 0))